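; BP_PointLight is a switchable point light that other code can turn on or off.
; The Switchon and SwitchOff events set the PointLight component's visibility and store the state in IsOn.
; IsSwithedOn returns that flag to callers.
; Disconnected leftover nodes cast the owner to BP_Button and reference its PointLights list, but they never run.
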(event `/Game/Blueprint/BPI_Switchable.SwitchOn`
  (`SceneComponent.SetVisibility` (`self.PointLight`) true false)
  (set `self.IsOn` true))

(event `/Game/Blueprint/BPI_Switchable.SwitchOff`
  (`SceneComponent.SetVisibility` (`self.PointLight`) false false)
  (set `self.IsOn` false))

(fn `IsSwithedOn`
  (returns (IsOn :type Boolean))
  (return (`self.IsOn`)))

(fn `UserConstructionScript`)